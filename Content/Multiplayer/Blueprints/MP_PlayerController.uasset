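; Multiplayer player controller that manages the match HUD for its local player.
; A ClientPostLogin event calls SetUpGameHud, which creates the W_MPHud widget and adds it to the viewport only on a local controller.
; That event then casts the game mode to MP_GameMode_Match, but no player-spawn logic follows despite its comment.
; EndPlay removes the stored HUD widget.
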(event `ClientPostLogin`
  ;[1 1 1] After login, set up ui and spawn player
  (`self.SetUpGameHud`)
  (cast `/Game/Multiplayer/Blueprints/GameModes/MP_GameMode_Match` (`GameplayStatics.GetGameMode`)))

(event `self.ReceiveEndPlay`
  (params (EndPlayReason :type "EEndPlayReason Enum" :default "Destroyed"))
  ;[1 1 1] After Leaving, remove hud
  (`Widget.RemoveFromParent` (`self.W_HUD`)))

(fn `SetUpGameHud`
  (if (`self.IsLocalPlayerController`)
    (bind _returnvalue (`|CreateWidget` "/Game/Multiplayer/Widgets/W_MPHud.W_MPHud_C" self))
    (bind _output_get (set `self.W_HUD` _returnvalue))
    (`UserWidget.AddToViewport` _output_get 0)))

(fn `UserConstructionScript`)