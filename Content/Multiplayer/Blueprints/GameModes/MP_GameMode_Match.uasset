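; Multiplayer match game mode that runs a loadout-selection countdown and restarts rounds when a team is wiped out.
; PostLogin sorts tagged PlayerStarts into two spawn lists, numbers each player and registers their controller.
; BeginPlay starts a looping countdown timer shown through the Steam game instance.
; Deaths shrink alive-team arrays; an empty one respawns everyone as mechs, choosing spawns by PlayerArray order, though teams are never populated here and StartRound is empty.
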(event `SRV_PlayerDeath`
  (params (`Player Controller` :type "/Game/Multiplayer/Blueprints/MP_PlayerController Object Reference"))
  (`self.K2_DestroyActor` (`Controller.K2_GetPawn` `Player Controller`))
  (if (`KismetArrayLibrary.Array_Contains` (`self.Team1`) `Player Controller`)
    (`KismetArrayLibrary.Array_RemoveItem` (`self.Team1Alive`) `Player Controller`)
    (else
      (`KismetArrayLibrary.Array_RemoveItem` (`self.Team2Alive`) `Player Controller`)))
  (`self.CheckRoundEnd`))

(event `self.ReceiveBeginPlay`
  (`self.SRV_StartLoadoutSelection`))

(event `SRV_StartLoadoutSelection`
  (bind _asmp_game_instance_steam (cast `/Game/Multiplayer/Blueprints/MP_GameInstance_Steam` (`GameplayStatics.GetGameInstance`)))
  (`/Game/Multiplayer/Blueprints/MP_GameInstance_Steam.ShowCountdownTimer` _asmp_game_instance_steam)
  (`KismetSystemLibrary.K2_SetTimer` null "RoundCountdown" 1.0 true))

(event `StartRound`
  ;[1 1 1] This will start the round
)

(event `RespawnPlayerEvent`
  (params (PlayerController :type "PlayerController Object Reference"))
  (bind _returnvalue (`Controller.K2_GetPawn` PlayerController))
  ;[1 1 1] Respawn player 1, 2 to spawn location
  (`/Engine/EditorBlueprintResources/StandardMacros.IsValid` _returnvalue
    (:`Is Valid`
      (`self.K2_DestroyActor` _returnvalue))
    (:`Is Not Valid`
      _))
  (if (== (`PlayerState.PlayerId` (`Controller.PlayerState` PlayerController)) (`PlayerState.PlayerId` (`KismetArrayLibrary.Array_Get` (`GameState.PlayerArray` (`GameplayStatics.GetGameState`)))))
    (bind _returnvalue_2 (`|SpawnActorFromClass` "/Game/Multiplayer/Blueprints/Characters/MP_Mech_Character.MP_Mech_Character_C" (`self.GetTransform` (`KismetArrayLibrary.Array_Get` (`self.Player1`))) "AdjustIfPossibleButAlwaysSpawn" "OverrideRootScale"))
    (`Controller.Possess` PlayerController _returnvalue_2)
    (else
      (bind _returnvalue_3 (`|SpawnActorFromClass` "/Game/Multiplayer/Blueprints/Characters/MP_Mech_Character.MP_Mech_Character_C" (`self.GetTransform` (`KismetArrayLibrary.Array_Get` (`self.Player2`))) "AdjustIfPossibleButAlwaysSpawn" "OverrideRootScale"))
      (`Controller.Possess` PlayerController _returnvalue_3))))

(event `self.K2_PostLogin`
  (params (NewPlayer :type "PlayerController Object Reference"))
  ;[1 1 1] Post login
  (`/Engine/EditorBlueprintResources/ActorMacros.Switch Has Authority`
    (:`Authority`
      (bind _outactors (`GameplayStatics.GetAllActorsOfClass` "/Script/Engine.PlayerStart"))
      (for _array_element _outactors
        (if (== (`PlayerStart.PlayerStartTag` _array_element) "Player1")
          (`KismetArrayLibrary.Array_AddUnique` (`self.Player1`) _array_element)
          (else
            (`KismetArrayLibrary.Array_AddUnique` (`self.Player2`) _array_element))))
      (bind _asmp_player_state (cast `/Game/Multiplayer/Blueprints/MP_PlayerState` (`Controller.PlayerState` NewPlayer)))
      ;;[1 1 1] Verifies same player order
      (set `/Game/Multiplayer/Blueprints/MP_PlayerState.PlayerNumber` (`KismetArrayLibrary.Array_Length` (`GameState.PlayerArray` (`GameplayStatics.GetGameState`))) _asmp_player_state)
      (bind _asmp_player_controller (cast `/Game/Multiplayer/Blueprints/MP_PlayerController` NewPlayer))
      (`/Game/Multiplayer/Blueprints/MP_PlayerController.ClientPostLogin` _asmp_player_controller)
      (`KismetArrayLibrary.Array_AddUnique` (`self.Players`) _asmp_player_controller))))

(fn `CheckRoundEnd`
  (if (== (`KismetArrayLibrary.Array_Length` (`self.Team1Alive`)) 0)
    (for _array_element (`self.Players`) :!label _label
      (`self.RespawnPlayerEvent` _array_element))
    (elif (== (`KismetArrayLibrary.Array_Length` (`self.Team2Alive`)) 0)
      (goto _label))))

(fn `RoundCountdown`
  (bind _asmp_game_instance_steam (cast `/Game/Multiplayer/Blueprints/MP_GameInstance_Steam` (`GameplayStatics.GetGameInstance`)))
  (if (== (`self.CountdownTimer`) 0.0)
    (`KismetSystemLibrary.K2_PauseTimer` null "RoundCountdown")
    (`/Game/Multiplayer/Blueprints/MP_GameInstance_Steam.HideCountdownTimer` _asmp_game_instance_steam)
    (set `self.CountdownTimer` (`self.LoadoutSelectionTime`))
    (else
      (set `self.CountdownTimer` (- (`self.CountdownTimer`) 1.0)))))

(fn `UserConstructionScript`)