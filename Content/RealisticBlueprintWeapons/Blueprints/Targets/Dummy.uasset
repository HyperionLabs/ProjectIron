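; Dummy is a moving target actor in the weapons pack that is knocked into the air when damaged.
; Until broken, Tick moves it by Direction scaled by delta time without sweeping, and the construction script sets its life span from Lifetime.
; Any damage sets IsBroken, stopping that movement, then enables gravity on the StaticMesh and applies a strong upward impulse.
; The Explode event is an empty stub.
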(event `self.ReceiveAnyDamage`
  (params (Damage :type "Float (single-precision)") (DamageType :type "DamageType Object Reference") (InstigatedBy :type "Controller Object Reference") (DamageCauser :type "Actor Object Reference"))
  (bind _staticmesh (`self.StaticMesh`))
  (set `self.IsBroken` true)
  (`PrimitiveComponent.SetEnableGravity` _staticmesh true)
  (`PrimitiveComponent.AddImpulse` _staticmesh (0.0 0.0 50000.0) "None" false))

(event `Explode`
  (params (Damage :type "Float (double-precision)")))

(event `self.ReceiveTick`
  (params (DeltaSeconds :type "Float (single-precision)"))
  (if (not (`self.IsBroken`))
    (`self.K2_SetActorLocation` (+ (* (`self.Direction`) DeltaSeconds) (`self.K2_GetActorLocation`)))))

(fn `UserConstructionScript`
  (`self.SetLifeSpan` (`self.lifetime`)))