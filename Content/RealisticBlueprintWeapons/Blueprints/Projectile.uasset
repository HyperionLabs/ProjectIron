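; Server-authoritative bullet actor that simulates ballistic flight, applying gravity and drag derived from caliber and mass, with wind left disconnected.
; Each tick line-traces along the velocity, then either moves the bullet or applies speed-scaled damage on impact.
; A data table matched on physical material picks the impact effect and resolves angle-based random ricochet or energy-based penetration.
; Lost energy becomes physics impulse, and movement can re-run within the same frame after a hit.
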(event Custom|CLI_DrawDebugLine
  (params (Start :type Vector :default "0, 0, 0") (End :type Vector :default "0, 0, 0") (TraceType :type EDrawDebugTrace%20Enum :default "None"))
  (Collision|LineTraceByChannel Start End "TraceTypeQuery1" false 0 TraceType))

(event Custom|SRV_SetMesh
  (Components|StaticMesh|SetStaticMesh (Variables|Default|GetProjectileMesh) (Variables|Default|GetMesh)))

(event EventBeginPlay
  (CallFunction|SRVSetMesh))

(event EventTick
  (params (DeltaSeconds :type Float%20%28single-precision%29))
  (Networking|SwitchHasAuthority
    (:Authority
      (Variables|Default|SetFrameBeginVelocityLength (Math|Vector|VectorLength (Variables|Default|GetVelocity)))
      (Variables|Default|SetFrameTravelDistance 0.0)
      (bind _output_get (Variables|Default|SetDeltaSeconds DeltaSeconds))
      (CallFunction|BulletMovement _output_get))))

(fn ConstructionScript
  (Variables|Default|SetInitialSpeed (Math|Vector|VectorLength (Variables|Default|GetVelocity)))
  (CallFunction|Initialize))

(fn ApplyGravity
  (params (DeltaSeconds :type Float%20%28single-precision%29))
  ;[1 1 1] Adds gravity to the velocity. 9.8m per second.
  (Networking|SwitchHasAuthority
    (:Authority
      (Variables|Default|SetVelocity (+ (* "0, 0,-980.000000" DeltaSeconds) (Variables|Default|GetVelocity))))))

(fn ApplyDrag
  (params (DeltaSeconds :type Float%20%28single-precision%29))
  (Variables|Default|SetVelocity (* (Variables|Default|GetVelocity) (* (- (Math|Vector|VectorLength (Variables|Default|GetVelocity)) (* (* DeltaSeconds (* (Math|Float|Power (/ (Math|Vector|VectorLength (Variables|Default|GetVelocity)) 1e+02) 2.0) (/ (Variables|Default|GetD) (Variables|Default|GetMassInKg)))) 1e+02)) (/ 1.0 (Math|Vector|VectorLength (Variables|Default|GetVelocity)))))))

(fn Trace
  (params (DeltaSeconds :type Float%20%28single-precision%29))
  (bind _returnvalue (Transformation|GetActorLocation))
  (bind _velocity (Variables|Default|GetVelocity))
  (bind _velocity_2 (Variables|Default|GetVelocity))
  (bind _debugtrace (Variables|Default|GetDebugTrace))
  (bind _initialspeed (Variables|Default|GetInitialSpeed))
  (bind _returnvalue_2 (Math|Vector|VectorLength _velocity))
  (bind _returnvalue_3 (* _velocity_2 DeltaSeconds))
  (bind _returnvalue_4 (/ _returnvalue_2 _initialspeed))
  (bind _returnvalue_5 (+ _returnvalue_3 _returnvalue))
  (bind _returnvalue_6 (Math|Color|Lerp(LinearColor) "(R=0.000000,G=1.000000,B=0.000000,A=1.000000)" "(R=1.000000,G=0.000000,B=0.000000,A=1.000000)" _returnvalue_4))
  ;[1 1 1] Here we're doing a line trace to see if we hit something
  (Networking|SwitchHasAuthority
    (:Authority
      (CallFunction|CLIDrawDebugLine _returnvalue _returnvalue_5 _debugtrace)
      (bind (_outhit _returnvalue_7) (Collision|LineTraceByChannel _returnvalue _returnvalue_5 "TraceTypeQuery1" false 0 _debugtrace false _returnvalue_6 _returnvalue_6))
      (return _returnvalue_7 _outhit))))

(fn MoveProjectile
  (params (DeltaSeconds :type Float%20%28single-precision%29))
  ;[1 1 1] Moving the projectile to its new location. Only server does this to prevent cheating
  (Networking|SwitchHasAuthority
    (:Authority
      (Transformation|SetActorLocation (+ (* (Variables|Default|GetVelocity) DeltaSeconds) (Transformation|GetActorLocation)) false false)
      (Transformation|SetActorRotation (Math|Conversions|RotationFromXVector (Math|Vector|Normalize (Variables|Default|GetVelocity)))))))

(fn Impact
  (params (InHit :type Hit%20Result%20Structure))
  (bind (_bblockinghit _binitialoverlap _time _location _impactpoint _normal _impactnormal _physmat _hitactor) (Collision|BreakHitResult InHit))
  (bind _returnvalue (* _impactnormal 0.1))
  (bind _returnvalue_2 (+ _location _returnvalue))
  (Game|Damage|ApplyDamage _hitactor (* (/ (Math|Vector|VectorLength (Variables|Default|GetVelocity)) (Variables|Default|GetInitialSpeed)) (Variables|Default|GetBaseDamage)) 0 0)
  (CallFunction|UpdateFrameMovement _returnvalue_2)
  ;[1 1 1] Move to impact location
  (Transformation|SetActorLocation _returnvalue_2 false false)
  (CallFunction|RicochetandPenetration InHit)
  (if (< (Variables|Default|GetFrameTravelDistance) (- (Variables|Default|GetFrameBeginVelocityLength) 3e+01))
    (Utilities|IsValid self
      (:Is%20Valid
        (CallFunction|BulletMovement (Variables|Default|GetDeltaSeconds))))))

(fn Initialize
  (Variables|Default|SetD (/ (* (* (Variables|Default|GetAirDensity) (Variables|Default|GetDrag)) (Math|Float|MultiplybyPi (Math|Float|Power (/ (/ (Variables|Default|GetCaliberDiameter) 1e+03) 2.0) 2.0))) 2.0))
  (Variables|Default|SetMassInKg (/ (Variables|Default|GetMass) 1e+03))
  ;[1 1 1] We need the initial speed to calculate the damage
  (Variables|Default|SetInitialSpeed (Math|Vector|VectorLength (Variables|Default|GetVelocity))))

(fn ApplyWind
  (params (Delta%20Seconds :type Float%20%28single-precision%29))
  (bind _worldwind (Variables|Default|GetWorldWind))
  (bind _returnvalue (Math|Vector|VectorLength _worldwind))
  (Variables|Default|SetVelocity (+ (* (Variables|Default|GetWorldWind) (- 1.0 (* (- _returnvalue (* (* Delta%20Seconds (* (Math|Float|Power (/ (Math|Vector|VectorLength (Variables|Default|GetWorldWind)) 1e+02) 2.0) (/ (* (Variables|Default|GetD) 2.0) (Variables|Default|GetMassInKg)))) 1e+02)) (/ 1.0 (+ _returnvalue 1.0))))) (Variables|Default|GetVelocity))))

(fn OnRepMesh)

(fn SpawnImpactEffect
  (params (Hit :type Hit%20Result%20Structure))
  (bind (_bblockinghit _binitialoverlap _time _location _impactpoint _normal _impactnormal) (Collision|BreakHitResult Hit))
  (bind _impacteffect (CallFunction|GetImpactEffect (.ImpactEffect (Utilities|Struct|BreakImpactBehavior (Variables|ImpactAndPenetration|GetImpactBehavior)))))
  (Game|SpawnActorfromClass _impacteffect (Math|Transform|MakeTransform _impactpoint (Math|Rotator|MakeRotfromX _impactnormal)) "AdjustIfPossibleButDontSpawnIfColliding" 0 0))

(fn RicochetandPenetration
  (params (Hit :type Hit%20Result%20Structure))
  (LocalVariables|SetHitResult Hit)
  ;[1 1 1] Loop impact behaviors.
  (bind _outrownames (DataTable|GetDataTableRowNames "/Game/RealisticBlueprintWeapons/Blueprints/ImpactBehaviorData.ImpactBehaviorData"))
  (bind _index (Utilities|FlowControl|ForLoopwithBreak 0 (- (Utilities|Array|Length _outrownames) -1) :!label _label)
    (:LoopBody
      ;[1 1 1] Find correct impact behavior
      (bind _returnvalue (Utilities|GetDataTableRow "/Game/RealisticBlueprintWeapons/Blueprints/ImpactBehaviorData.ImpactBehaviorData" (Utilities|Array|Get(acopy) _outrownames _index))
        (:then
          (if (Utilities|Enum|Equal(Enum) (.MaterialName (Utilities|Struct|BreakImpactBehavior _returnvalue)) (Utilities|String|ToString(Object) (.PhysMat (Collision|BreakHitResult (LocalVariables|GetHitResult)))))
            (Variables|ImpactAndPenetration|SetImpactBehavior _returnvalue)
            (Variables|Default|SetImpactBehaviorFound true)
            (Utilities|FlowControl|Sequence
              (:then_0
                (goto _label Break))
              (:then_1
                (CallFunction|SpawnImpactEffect (LocalVariables|GetHitResult))
                (if (and (< (+ (Math|Random|RandomFloatinRange 0.0 (- (.MaximumRicochetAngle (Utilities|Struct|BreakImpactBehavior (Variables|ImpactAndPenetration|GetImpactBehavior))) (.MinimumRicochetAngle (Utilities|Struct|BreakImpactBehavior (Variables|ImpactAndPenetration|GetImpactBehavior))))) (Math|Float|Absolute(Float) (Class|KismetMathLibrary|DegAsin (Math|Vector|DotProduct (.ImpactNormal (Collision|BreakHitResult (LocalVariables|GetHitResult))) (Math|Vector|Normalize (Variables|Default|GetVelocity)))))) (.MaximumRicochetAngle (Utilities|Struct|BreakImpactBehavior (Variables|ImpactAndPenetration|GetImpactBehavior)))) (Variables|Default|GetDoesRicochet))
                  (bind _joule_loss (CallFunction|Ricochet (.ImpactNormal (Collision|BreakHitResult (LocalVariables|GetHitResult))) (Math|Float|Absolute(Float) (Class|KismetMathLibrary|DegAsin (Math|Vector|DotProduct (.ImpactNormal (Collision|BreakHitResult (LocalVariables|GetHitResult))) (Math|Vector|Normalize (Variables|Default|GetVelocity)))))))
                  (CallFunction|AddImpulsetoImpact (.HitComponent (Collision|BreakHitResult (LocalVariables|GetHitResult))) (* (* (.ImpactNormal (Collision|BreakHitResult (LocalVariables|GetHitResult))) -1.0) _joule_loss) (.ImpactPoint (Collision|BreakHitResult (LocalVariables|GetHitResult))))
                  (else
                    (bind _joule_loss_2 (CallFunction|Penetration (LocalVariables|GetHitResult)))
                    (CallFunction|AddImpulsetoImpact (.HitComponent (Collision|BreakHitResult (LocalVariables|GetHitResult))) (* (Math|Vector|Normalize (Variables|Default|GetVelocity)) _joule_loss_2) (.ImpactPoint (Collision|BreakHitResult (LocalVariables|GetHitResult))))))))))))
    (:Completed
      ;[1 1 1] Kill projectile if no impact behavior is found
      (if (Variables|Default|GetImpactBehaviorFound)
        (Variables|Default|SetImpactBehaviorFound false)
        (else
          (Game|SpawnActorfromClass "/Game/RealisticBlueprintWeapons/Blueprints/WeaponEffects/Impact.Impact_C" (Math|Transform|MakeTransform (.ImpactPoint (Collision|BreakHitResult (LocalVariables|GetHitResult))) (Math|Rotator|MakeRotfromX (.ImpactNormal (Collision|BreakHitResult (LocalVariables|GetHitResult))))) "AdjustIfPossibleButDontSpawnIfColliding" 0 0)
          (bind _joules (CallFunction|GetJoules))
          (CallFunction|AddImpulsetoImpact (.HitComponent (Collision|BreakHitResult (LocalVariables|GetHitResult))) (* (Math|Vector|Normalize (Variables|Default|GetVelocity)) _joules) (.ImpactPoint (Collision|BreakHitResult (LocalVariables|GetHitResult))))
          (Actor|DestroyActor))))))

(fn Penetration
  (params (Hit%20result :type Hit%20Result%20Structure))
  (bind (_bblockinghit _binitialoverlap _time _location _impactpoint _normal _impactnormal _physmat _hitactor _hitcomponent) (Collision|BreakHitResult Hit%20result))
  (bind _returnvalue (Transformation|GetActorLocation))
  (bind _joules (CallFunction|GetJoules))
  (LocalVariables|SetPreImpactJoule _joules)
  ;[1 1 1] Find other side of object being hit.
  (bind (_outhit _returnvalue_2) (Collision|LineTraceByChannel (+ (* (Math|Vector|Normalize (Variables|Default|GetVelocity)) (/ (* (* (Variables|Default|GetMassInKg) 0.5) (Math|Float|Power (/ (Math|Vector|VectorLength (Variables|Default|GetVelocity)) 1e+02) 2.0)) (.JoulePerCm (Utilities|Struct|BreakImpactBehavior (Variables|ImpactAndPenetration|GetImpactBehavior))))) _returnvalue) _returnvalue "TraceTypeQuery1" false (LocalVariables|GetActorsToIgnore) "None" :!label _label))
  (if _returnvalue_2
    (if (== _hitcomponent (.HitComponent (Collision|BreakHitResult _outhit)))
      (Variables|Default|SetVelocity (* (Variables|Default|GetVelocity) (/ (* (/ 1e+02 (/ (* (* (Variables|Default|GetMassInKg) 0.5) (Math|Float|Power (/ (Math|Vector|VectorLength (Variables|Default|GetVelocity)) 1e+02) 2.0)) (.JoulePerCm (Utilities|Struct|BreakImpactBehavior (Variables|ImpactAndPenetration|GetImpactBehavior))))) (- (/ (* (* (Variables|Default|GetMassInKg) 0.5) (Math|Float|Power (/ (Math|Vector|VectorLength (Variables|Default|GetVelocity)) 1e+02) 2.0)) (.JoulePerCm (Utilities|Struct|BreakImpactBehavior (Variables|ImpactAndPenetration|GetImpactBehavior)))) (Math|Vector|VectorLength (- (Transformation|GetActorLocation) (.Location (Collision|BreakHitResult _outhit)))))) 1e+02)))
      (Transformation|SetActorLocation (+ (.Location (Collision|BreakHitResult _outhit)) (.Normal (Collision|BreakHitResult _outhit))) false false)
      (bind _joules_2 (CallFunction|GetJoules))
      (return (- (LocalVariables|GetPreImpactJoule) _joules_2))
      (else
        (Utilities|Array|AddUnique (LocalVariables|GetActorsToIgnore) (.HitActor (Collision|BreakHitResult _outhit)))
        (goto _label)))
    (else
      (CallFunction|AddImpulsetoImpact _hitcomponent (* (Math|Vector|Normalize (Variables|Default|GetVelocity)) (LocalVariables|GetPreImpactJoule)) _impactpoint)
      ;[1 1 1] No penetration, bullet dies
      (Actor|DestroyActor))))

(fn Ricochet
  (params (ImpactNormal :type Vector) (ImpactAngle :type Float%20%28single-precision%29))
  (bind _joules (CallFunction|GetJoules))
  (LocalVariables|SetPre%20impact%20Joules _joules)
  (Variables|Default|SetVelocity (* (Math|Vector|MirrorVectorbyNormal (Variables|Default|GetVelocity) ImpactNormal) (- 1.0 (/ ImpactAngle 1e+02))))
  (bind _joules_2 (CallFunction|GetJoules))
  (return (- (LocalVariables|GetPre%20impact%20Joules) _joules_2)))

(fn GetImpactEffect
  (params (Impact :type ImpactEffects%20Enum))
  (switch Utilities|FlowControl|Switch|SwitchonImpactEffects Impact
    (:NewEnumerator0
      (LocalVariables|SetLocal_impactEffect "/Game/RealisticBlueprintWeapons/Blueprints/WeaponEffects/Impact.Impact_C"))
    (:NewEnumerator1
      (LocalVariables|SetLocal_impactEffect "/Game/RealisticBlueprintWeapons/Blueprints/WeaponEffects/MuzzleEffect.MuzzleEffect_C"))
    (:NewEnumerator2
      (LocalVariables|SetLocal_impactEffect "/Game/RealisticBlueprintWeapons/Blueprints/WeaponEffects/BaseWeaponEffect.BaseWeaponEffect_C"))
    (:NewEnumerator3
      (LocalVariables|SetLocal_impactEffect "/Game/RealisticBlueprintWeapons/Blueprints/WeaponEffects/BaseWeaponEffect.BaseWeaponEffect_C")))
  (return (LocalVariables|GetLocal_impactEffect)))

(fn GetJoules
  (return (* (* (Variables|Default|GetMassInKg) 0.5) (Math|Float|Power (/ (Math|Vector|VectorLength (Variables|Default|GetVelocity)) 1e+02) 2.0))))

(fn AddImpulsetoImpact
  (params (Actor%20Component :type Primitive%20Component%20Object%20Reference) (Impulse :type Vector) (Location :type Vector))
  (if (Physics|IsSimulatingPhysics Actor%20Component "None")
    (Physics|AddImpulseatLocation Actor%20Component Impulse Location "None")))

(fn UpdateFrameMovement
  (params (MoveToLocation :type Vector))
  (Variables|Default|SetFrameTravelDistance (+ (Math|Vector|VectorLength (- MoveToLocation (Transformation|GetActorLocation))) (Variables|Default|GetFrameTravelDistance))))

(fn BulletMovement
  (params (DeltaSeconds :type Float%20%28single-precision%29))
  (bind (_returnvalue _outhit) (CallFunction|Trace DeltaSeconds))
  (if _returnvalue
    (CallFunction|Impact _outhit)
    (else
      (CallFunction|MoveProjectile (Variables|Default|GetDeltaSeconds))
      (CallFunction|ApplyGravity (Variables|Default|GetDeltaSeconds))
      (CallFunction|ApplyDrag (Variables|Default|GetDeltaSeconds)))))