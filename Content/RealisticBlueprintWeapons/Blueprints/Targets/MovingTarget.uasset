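; MovingTarget is a shootable destructible target actor that shatters when it takes any damage.
; AnyDamage calls Explode, which sets IsBroken, enables gravity, adds an upward impulse and applies massively scaled radius damage at the actor's location to fracture the Destructible.
; The construction script sets the life span from Lifetime.
; Despite the name it does not move itself: the authority-only movement logic is disconnected and multiplies MovementVector by zero.
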(event `self.ReceiveAnyDamage`
  (params (Damage :type "Float (single-precision)") (DamageType :type "DamageType Object Reference") (InstigatedBy :type "Controller Object Reference") (DamageCauser :type "Actor Object Reference"))
  (`self.Explode` Damage))

(event `Explode`
  (params (Damage :type "Float (double-precision)"))
  (bind _destructible (`self.Destructible`))
  (set `self.IsBroken` true)
  (`PrimitiveComponent.SetEnableGravity` (`self.Destructible`) true)
  (`PrimitiveComponent.AddImpulse` _destructible (0.0 0.0 5000.0) "None" false)
  (`DestructibleComponent.ApplyRadiusDamage` _destructible (* Damage 99999.0) (`self.K2_GetActorLocation` self) 1.0 3000.0 true))

(event `self.ReceiveTick`
  (params (DeltaSeconds :type "Float (single-precision)")))

(fn `UserConstructionScript`
  (`self.SetLifeSpan` self (`self.Lifetime`)))