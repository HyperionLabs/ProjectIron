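; Crosshair is a HUD Blueprint that draws a small first-person crosshair texture at the center of the screen.
; On BeginPlay it casts the owning pawn to TestCharacter and caches it as Player.
; Each DrawHUD calls IsAimingMessage on the pawn, but the branch is fixed to true and the negated result is unused, so the crosshair shows regardless of aiming.
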(event `self.ReceiveBeginPlay`
  (bind _astest_character (cast `/Game/RealisticBlueprintWeapons/Blueprints/TestCharacter` (`self.GetOwningPawn`)))
  (set `self.Player` _astest_character))

(event `self.ReceiveDrawHUD`
  (params (SizeX :type Integer) (SizeY :type Integer))
  (bind _isaiming (message `/Game/Multiplayer/Blueprints/Weapons/WeaponSystems/BPI_Weaponuser.IsAiming` (`self.GetOwningPawn`)))
  (if true
    (`self.DrawTexture` "/Game/RealisticBlueprintWeapons/Materials/Textures/FirstPersonCrosshair.FirstPersonCrosshair" (`KismetMathLibrary.Conv_IntToDouble` (- (/ SizeX 2) 8)) (`KismetMathLibrary.Conv_IntToDouble` (- (/ SizeY 2) 8)) 16.0 16.0 0.0 0.0 1.0 1.0 (make `LinearColor` 1.0 1.0 1.0 1.0))))

(fn `UserConstructionScript`)