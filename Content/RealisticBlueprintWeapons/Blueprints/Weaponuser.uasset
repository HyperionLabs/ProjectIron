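; Weapon user component that lets its owning Character hold and operate a single equipped weapon.
; EquipWeapon stores the weapon and socket, and the EquippedWeapon RepNotify snaps it to the character mesh, sets its owner and disables physics.
; SRV-prefixed events forward firing, trigger, reload, jam-fix and fire-mode input to the weapon.
; CLI_Recoil applies recoil as pitch and yaw input on player controller 0.
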(event `SRV_ShootToLocation`
  (params (`Crosshair Location` :type "Vector Structure") (ShootToLocation :type Boolean))
  (`/Game/Sandbox/Weapons/BaseWeapon.SRV_ShootToLocation` (`self.EquippedWeapon`) `Crosshair Location` ShootToLocation))

(event `SRV_PullTrigger`
  (params (TargetLocation :type "Vector Structure") (`Shoot to Location` :type Boolean))
  (bind _equippedweapon (`self.EquippedWeapon`))
  ;[1 0.01675 0] Pass events to the weapon
  (`/Game/Sandbox/Weapons/BaseWeapon.SetIsTriggerPulled` _equippedweapon true)
  (`/Game/Sandbox/Weapons/BaseWeapon.SRV_Fire` _equippedweapon TargetLocation `Shoot to Location`))

(event `SRV_ReleaseTrigger`
  ;[1 0.01675 0] Pass events to the weapon
  (`/Game/Sandbox/Weapons/BaseWeapon.SetIsTriggerPulled` (`self.EquippedWeapon`) false))

(event `SRV_Reload`
  ;[1 0.01675 0] Pass events to the weapon
  (`/Game/Sandbox/Weapons/BaseWeapon.ReloadEvent` (`self.EquippedWeapon`)))

(event `SRV_FixJam`
  ;[1 0.01675 0] Pass events to the weapon
  (`/Game/Sandbox/Weapons/BaseWeapon.SetIsJammed` (`self.EquippedWeapon`) false))

(event `SRV_FireModeStep`
  ;[1 0.01675 0] Pass events to the weapon
  (`/Game/Sandbox/Weapons/BaseWeapon.FireModeStep` (`self.EquippedWeapon`)))

(event `CLI_Recoil`
  (params (VerticalRecoil :type "Float (double-precision)") (HorizontalRecoil :type "Float (double-precision)"))
  (bind _returnvalue (`GameplayStatics.GetPlayerController` 0))
  (`PlayerController.AddPitchInput` _returnvalue VerticalRecoil)
  (`PlayerController.AddYawInput` _returnvalue HorizontalRecoil))

(fn `Equip Weapon`
  (params (Weapon :type "/Game/Sandbox/Weapons/BaseWeapon Object Reference") (SocketName :type Name))
  (set `self.WeaponSocketName` SocketName)
  (set `self.EquippedWeapon` Weapon))

(fn `GetWeapon`
  (returns (EquippedWeapon :type "/Game/Sandbox/Weapons/BaseWeapon Object Reference"))
  (return (`self.EquippedWeapon`)))

(fn `HasWeaponEquipped`
  (returns (HasWeaponEquipped :type Boolean))
  (return (`KismetSystemLibrary.IsValid` (`self.EquippedWeapon`))))

(fn `OnRep_EquippedWeapon`
  (bind _equippedweapon (`self.EquippedWeapon`))
  (bind _equippedweapon_2 (`self.EquippedWeapon`))
  (bind _ascharacter (cast `Character` (`self.GetOwner`)))
  (`/Engine/EditorBlueprintResources/StandardMacros.IsValid` _equippedweapon
    (:`Is Valid`
      (`Actor.K2_AttachRootComponentTo` _equippedweapon (`Character.Mesh` _ascharacter) (`self.WeaponSocketName`) "SnapToTarget" true)
      (set `/Game/Sandbox/Weapons/BaseWeapon.OwningPlayer` _ascharacter _equippedweapon_2)
      (set `/Game/Sandbox/Weapons/BaseWeapon.PhysicsEnabled` false _equippedweapon_2))))