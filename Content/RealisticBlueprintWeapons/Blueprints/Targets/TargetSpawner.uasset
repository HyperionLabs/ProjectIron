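; TargetSpawner is an actor that continuously spawns moving Dummy targets at its own transform.
; On BeginPlay, only the authority starts an endless loop that waits a random delay within the SpawnRate range, spawns a Dummy, then repeats.
; Each Dummy receives a Lifetime and a Direction vector, built from a random horizontal direction scaled by a random speed within MinMaxSpeed.
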(event `self.ReceiveBeginPlay`
  (bind (_x _y) (`KismetMathLibrary.BreakVector2D` (`self.SpawnRate`)))
  (bind (_x_2 _y_2) (`KismetMathLibrary.BreakVector2D` (`self.MinMaxSpeed`)))
  (`/Engine/EditorBlueprintResources/ActorMacros.Switch Has Authority`
    (:`Authority`
      (`KismetSystemLibrary.RetriggerableDelay` (`KismetMathLibrary.RandomFloatInRange` _x _y) :!label _label)
      (`|SpawnActorFromClass` "/Game/RealisticBlueprintWeapons/Blueprints/Targets/Dummy.Dummy_C" (`self.GetTransform` self) "Undefined" "OverrideRootScale" null (`self.Lifetime`) (* (`KismetMathLibrary.Normal` (`KismetMathLibrary.MakeVector` (.x (`KismetMathLibrary.RandomUnitVector`)) (.y (`KismetMathLibrary.RandomUnitVector`)))) (`KismetMathLibrary.RandomFloatInRange` _x_2 _y_2)))
      (goto _label))))

(event `self.ReceiveTick`
  (params (DeltaSeconds :type "Float (single-precision)")))

(fn `UserConstructionScript`)