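; Multiplayer game mode that handles player login and respawns for two player slots.
; On server post-login, it sorts PlayerStarts by tag into Player1 and Player2 lists, numbers the PS_MP player state by join count and calls ClientPostLogin on PC_MP.
; Respawn destroys the controlled pawn, then spawns and possesses a Sandbox3rdPersonCharacter at that slot's first start, treating the first PlayerArray entry as player one.
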(event `RespawnPlayerEvent`
  (params (PlayerController :type "PlayerController Object Reference"))
  ;[1 1 1] Respawn player 1, 2 to spawn location
  (`self.K2_DestroyActor` (`Controller.K2_GetPawn` PlayerController))
  (if (== (`PlayerState.PlayerId` (`KismetArrayLibrary.Array_Get` (`GameState.PlayerArray` (`GameplayStatics.GetGameState`)))) (`PlayerState.PlayerId` (`Controller.PlayerState` PlayerController)))
    (bind _returnvalue (`|SpawnActorFromClass` "/Game/Sandbox/Characters/Sandbox3rdPersonCharacter.Sandbox3rdPersonCharacter_C" (`self.GetTransform` (`KismetArrayLibrary.Array_Get` (`self.Player1`))) "AdjustIfPossibleButAlwaysSpawn" "OverrideRootScale"))
    (`Controller.Possess` PlayerController _returnvalue)
    (else
      (bind _returnvalue_2 (`|SpawnActorFromClass` "/Game/Sandbox/Characters/Sandbox3rdPersonCharacter.Sandbox3rdPersonCharacter_C" (`self.GetTransform` (`KismetArrayLibrary.Array_Get` (`self.Player2`))) "AdjustIfPossibleButAlwaysSpawn" "OverrideRootScale"))
      (`Controller.Possess` PlayerController _returnvalue_2))))

(event `self.K2_PostLogin`
  (params (NewPlayer :type "PlayerController Object Reference"))
  ;[1 1 1] Post login
  (`/Engine/EditorBlueprintResources/ActorMacros.Switch Has Authority`
    (:`Authority`
      (bind _outactors (`GameplayStatics.GetAllActorsOfClass` "/Script/Engine.PlayerStart"))
      (for _array_element _outactors
        (if (== (`PlayerStart.PlayerStartTag` _array_element) "Player1")
          (`KismetArrayLibrary.Array_AddUnique` (`self.Player1`) _array_element)
          (else
            (`KismetArrayLibrary.Array_AddUnique` (`self.Player2`) _array_element))))
      (bind _asps_mp (cast `/Game/Multiplayer/Blueprints/PS_MP` (`Controller.PlayerState` NewPlayer)))
      ;;[1 1 1] Verifies same player order
      (set `/Game/Multiplayer/Blueprints/PS_MP.PlayerNumber` (`KismetArrayLibrary.Array_Length` (`GameState.PlayerArray` (`GameplayStatics.GetGameState`))) _asps_mp)
      (bind _aspc_mp (cast `/Game/Multiplayer/Blueprints/PC_MP` NewPlayer))
      (`/Game/Multiplayer/Blueprints/PC_MP.ClientPostLogin` _aspc_mp))))

(fn `UserConstructionScript`)