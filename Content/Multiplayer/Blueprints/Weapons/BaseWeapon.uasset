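; Base multiplayer weapon with single, burst and full-auto fire, ammo, reloading and socketed attachments.
; SRV_Fire handles burst and full-auto timing with retriggerable delays, while authority-gated functions fire either hitscan traces or physical-parameter projectiles with spread, zeroing and multi-shot blasts.
; FindMuzzle aims from the weapon or muzzle attachment socket; only projectile shots can jam.
; Each shot sets random kick, which Tick interpolates and sends to the owner's weapon component.
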(event `self.ReceiveTick`
  (params (DeltaSeconds :type "Float (single-precision)"))
  ;[1 1 1] Setting timers for single shot or burst shot.
  (set `self.TimeSinceLastShot` (+ DeltaSeconds (`self.TimeSinceLastShot`)))
  (set `self.TimeSinceLastBurst` (+ DeltaSeconds (`self.TimeSinceLastBurst`)))
  (`self.DoRecoil`))

(event `SRV_ShootToLocation`
  (params (`Crosshair Location` :type "Vector Structure") (ShootToLocation :type Boolean))
  (set `self.CrosshairLocation` `Crosshair Location`)
  (set `self.ShootToLocation` ShootToLocation))

(event `SRV_Fire`
  (params (`Crosshair Location` :type "Vector Structure") (`Shoot to Location` :type Boolean) (`Owner Camera` :type "CameraComponent Object Reference"))
  ;[1 1 1] Fire weapon
  (set `self.CrosshairLocation` `Crosshair Location`)
  (set `self.OwnerCamera` `Owner Camera`)
  (set `self.ShootToLocation` `Shoot to Location`)
  (if (not (`self.IsReloading`))
    (switch `/Game/RealisticBlueprintWeapons/Blueprints/FireModes` (`self.CurrentFireMode`)
      (:`NewEnumerator0`
        ;[1 1 1] Single shot
        (`/Engine/EditorBlueprintResources/StandardMacros.IsValid` self
          (:`Is Valid`
            (`self.Fire`))))
      (:`NewEnumerator1`
        ;[1 1 1] No delay inside functions in UE4, loop placed here
        (if (> (`self.TimeSinceLastBurst`) (`self.BurstDelay`))
          (set `self.TimeSinceLastBurst` 0.0)
          (if (> (`self.BurstCount`) (`self.CurrentShotInBurst`)) :!label _label
            (`self.Fire`)
            (`KismetSystemLibrary.RetriggerableDelay` (`self.FireRateBurst`))
            (goto _label)
            (else
              (set `self.CurrentShotInBurst` 0)))))
      (:`NewEnumerator2`
        ;[1 1 1] No delay inside functions in UE4, loop placed here
        (if (`self.TriggerPulled`) :!label _label_2
          (`self.Fire`)
          (`KismetSystemLibrary.RetriggerableDelay` (`self.FireRateFullAuto`))
          (goto _label_2))))))

(event `self.ReceiveDestroyed`
  (`self.DestroyAttachments`))

(event `ReloadEvent`
  ;[1 1 1] Reload
  (set `self.IsReloading` true)
  (`KismetSystemLibrary.Delay` (`self.ReloadTime`))
  (`self.Reload`))

(event `ShotCosmetics`
  ;[1 1 1] Visual effects and sound
  (bind _returnvalue (`|SpawnActorFromClass` (`self.MuzzleFlash`) (`self.MuzzleSocketTransform`) "AdjustIfPossibleButDontSpawnIfColliding" "OverrideRootScale"))
  (`GameplayStatics.SpawnEmitterAttached` (`/Game/RealisticBlueprintWeapons/Blueprints/WeaponEffects/BaseWeaponEffect.Particle` _returnvalue) (`self.Weapon`) (`self.MuzzleName`) (0.0 0.0 0.0) (struct) "SnapToTarget"))

(fn `Attach`
  (params (Attachment :type "/Game/RealisticBlueprintWeapons/Blueprints/Attachments/BaseAttachment Object Reference"))
  (bind _attachtosocket (`/Game/RealisticBlueprintWeapons/Blueprints/Attachments/BaseAttachment.AttachToSocket` Attachment))
  (`/Game/RealisticBlueprintWeapons/Blueprints/Attachments/BaseAttachment.Attached` Attachment self)
  (`KismetArrayLibrary.Array_Add` (`self.Attachments`) Attachment)
  (if (and (`/Game/RealisticBlueprintWeapons/Blueprints/Attachments/BaseAttachment.IsVisual` Attachment) (`SceneComponent.DoesSocketExist` (`self.Weapon`) _attachtosocket))
    (`self.K2_AttachRootComponentTo` Attachment (`self.Weapon`) _attachtosocket "KeepRelativeOffset" true)))

(fn `DestroyAttachments`
  (`/Engine/EditorBlueprintResources/ActorMacros.Switch Has Authority`
    (:`Authority`
      (for _array_element (`self.Attachments`)
        (`self.Detach` _array_element)
        (`self.K2_DestroyActor` _array_element)))))

(fn `Detach`
  (params (Attachment :type "/Game/RealisticBlueprintWeapons/Blueprints/Attachments/BaseAttachment Object Reference"))
  (`/Game/RealisticBlueprintWeapons/Blueprints/Attachments/BaseAttachment.Detached` Attachment self))

(fn `DoRecoil`
  (bind _owningplayer (`self.OwningPlayer`))
  (bind _currentverticalrecoil (`self.CurrentVerticalRecoil`))
  (bind _currenthorisontalrecoil (`self.CurrentHorisontalRecoil`))
  (bind _returnvalue (`KismetMathLibrary.FInterpTo` _currenthorisontalrecoil (`self.TargetHorisontalRecoil`) (`GameplayStatics.GetWorldDeltaSeconds`) 20.0))
  (bind _returnvalue_2 (`KismetMathLibrary.FInterpTo` _currentverticalrecoil (`self.TargetVerticalRecoil`) (`GameplayStatics.GetWorldDeltaSeconds`) 20.0))
  (bind _returnvalue_3 (- _returnvalue _currenthorisontalrecoil))
  (bind _returnvalue_4 (- _returnvalue_2 _currentverticalrecoil))
  (`/Engine/EditorBlueprintResources/ActorMacros.Switch Has Authority`
    (:`Authority`
      ;[1 1 1] Don't call unless you have some recoil to do
      (if (or (!= _returnvalue_4 0.0) (!= _returnvalue_3 0.0))
        (if (`KismetSystemLibrary.DoesImplementInterface` _owningplayer "/Game/RealisticBlueprintWeapons/Blueprints/BPI_Weaponuser.BPI_Weaponuser_C")
          (bind _weaponuser (message `/Game/RealisticBlueprintWeapons/Blueprints/BPI_Weaponuser.GetWeaponComponent` _owningplayer))
          (`/Game/RealisticBlueprintWeapons/Blueprints/Weaponuser.CLI_Recoil` _weaponuser _returnvalue_4 _returnvalue_3)
          (set `self.CurrentVerticalRecoil` _returnvalue_2)
          (set `self.CurrentHorisontalRecoil` _returnvalue))))))

(fn `FindMuzzle`
  (bind _returnvalue (`SceneComponent.GetSocketTransform` (`self.Weapon`) (`self.MuzzleName`) "RTS_World"))
  (bind _rotation (.rotation _returnvalue))
  (bind _returnvalue_2 (`SceneComponent.GetSocketTransform` (`/Game/RealisticBlueprintWeapons/Blueprints/Attachments/BaseAttachment.Mesh` (`self.MuzzleAttachment`)) (`self.AlternativeMuzzleName`) "RTS_World"))
  (bind _returnvalue_3 (`KismetMathLibrary.FindLookAtRotation` (.location _returnvalue) (`self.CrosshairLocation`)))
  (bind _rotation_2 (.rotation _returnvalue_2))
  (bind _returnvalue_4 (`KismetMathLibrary.FindLookAtRotation` (.location _returnvalue_2) (`self.CrosshairLocation`)))
  (if (`self.UseAlternativeMuzzle`)
    (if (`self.ShootToLocation`)
      (set `self.ShotForwardVector` (`KismetMathLibrary.GetForwardVector` _returnvalue_4))
      (set `self.ShotForwardRotation` _returnvalue_4)
      (else
        (set `self.ShotForwardVector` (`KismetMathLibrary.GetForwardVector` _rotation_2))
        (set `self.ShotForwardRotation` _rotation_2)))
    (set `self.MuzzleSocketTransform` _returnvalue_2)
    (else
      (if true
        (set `self.ShotForwardVector` (`KismetMathLibrary.GetForwardVector` _returnvalue_3))
        (set `self.ShotForwardRotation` _returnvalue_3)
        (else
          (set `self.ShotForwardVector` (`KismetMathLibrary.GetForwardVector` _rotation))
          (set `self.ShotForwardRotation` _rotation)))
      (set `self.MuzzleSocketTransform` _returnvalue))))

(fn `Fire`
  (`/Engine/EditorBlueprintResources/ActorMacros.Switch Has Authority`
    (:`Authority`
      (bind _hasammo (`self.HasAmmo`))
      (if _hasammo
        (switch `/Game/RealisticBlueprintWeapons/Blueprints/FireModes` (`self.CurrentFireMode`)
          (:`NewEnumerator0`
            (`self.FireSingle`))
          (:`NewEnumerator1`
            (`self.FireBurst`))
          (:`NewEnumerator2`
            (`self.FireFullAuto`)))
        (else
          (`self.TriggerNoAmmo`))))))

(fn `FireBurst`
  (`/Engine/EditorBlueprintResources/ActorMacros.Switch Has Authority`
    (:`Authority`
      (set `self.CurrentShotInBurst` (+ (`self.CurrentShotInBurst`) 1))
      (if (`self.Hitscan`)
        (`self.HitscanFire`)
        (else
          (`self.Try Spawn Projectile`))))))

(fn `FireFullAuto`
  (`/Engine/EditorBlueprintResources/ActorMacros.Switch Has Authority`
    (:`Authority`
      (if (`self.Hitscan`)
        (`self.HitscanFire`)
        (else
          (`self.Try Spawn Projectile`))))))

(fn `FireModeStep`
  (switch `/Game/RealisticBlueprintWeapons/Blueprints/FireModes` (`self.CurrentFireMode`)
    (:`NewEnumerator0`
      (`self.Set Fire Mode Burst`))
    (:`NewEnumerator1`
      (`self.Set Fire Mode FullAuto`))
    (:`NewEnumerator2`
      (`self.SetFireModeSingle`))))

(fn `FireSingle`
  (`/Engine/EditorBlueprintResources/ActorMacros.Switch Has Authority`
    (:`Authority`
      (if (>= (`self.TimeSinceLastShot`) (`self.FireRateSingleShot`))
        (if (`self.Hitscan`)
          (`self.HitscanFire`)
          (else
            (`self.Try Spawn Projectile`)))))))

(fn `GetADSCameraLocation`
  (params (CameraSocketName :type Name))
  (returns (SocketLocation :type "Vector Structure"))
  (return (`SceneComponent.GetSocketLocation` (`self.Weapon`) CameraSocketName)))

(fn `GetHorisontalKick`
  (returns (HorisontalKick :type "Float (double-precision)"))
  (bind (_x _y) (`KismetMathLibrary.BreakVector2D` (`self.HorisontalKick`)))
  (set `self.CurrentHorisontalRecoil` 0.0)
  (return (`KismetMathLibrary.RandomFloatInRange` _x _y)))

(fn `GetVerticalKick`
  (returns (VerticalKick :type "Float (double-precision)"))
  (bind (_x _y) (`KismetMathLibrary.BreakVector2D` (`self.VerticalKick`)))
  (set `self.CurrentVerticalRecoil` 0.0)
  (return (* (`KismetMathLibrary.RandomFloatInRange` _x _y) -1.0)))

(fn `HasAmmo`
  (returns (HasAmmo :type Boolean))
  (return (> (`self.CurrentAmmo`) 0)))

(fn `HitscanFire`
  (bind _ownercamera (`self.OwnerCamera`))
  (bind _blastprojectilecount (`self.BlastProjectileCount`))
  (`self.FindMuzzle`)
  (`/Engine/EditorBlueprintResources/ActorMacros.Switch Has Authority`
    (:`Authority`
      (set `self.TimeSinceLastShot` 0.0)
      (set `self.CurrentAmmo` (- (`self.CurrentAmmo`) 1))
      (`self.ShotCosmetics`)
      (`self.SetRecoil`)
      (if (`self.SpreadHitscan`)
        (set `self.ShotLocation` (+ (`SceneComponent.K2_GetComponentLocation` _ownercamera) (* (`KismetMathLibrary.RandomUnitVectorInConeWithYawAndPitch` (`SceneComponent.GetForwardVector` _ownercamera) 10.0 10.0) 99999999.0)) :!label _label)
        (bind _outhit (`KismetSystemLibrary.LineTraceSingle` :`Start` (.location (`self.MuzzleSocketTransform`)) :`End` (`self.ShotLocation`) :`TraceChannel` "TraceTypeQuery1" :`DrawDebugType` (`self.DebugTrace`) :`TraceColor` (struct :`R` 1.0 :`B` 0.504 :`A` 1.0) :`TraceHitColor` (struct :`B` 1.0 :`A` 1.0) :!label _label_2))
        (bind _ascharacter (cast `Character` (`.HitActor` (`GameplayStatics.BreakHitResult` _outhit)))
          (:`then`
            (`GameplayStatics.ApplyDamage` _ascharacter (`self.BaseDamage`) (`GameplayStatics.GetPlayerController` 0) self))
          (:`CastFailed`
            _))
        (if (and (> _blastprojectilecount 0) (< (`self.CurrentBlastCount`) _blastprojectilecount))
          (set `self.CurrentBlastCount` (+ (`self.CurrentBlastCount`) 1))
          (goto _label)
          (else
            _))
        (else
          (set `self.ShotLocation` (`self.CrosshairLocation`))
          (goto _label_2)))
      (set `self.CurrentBlastCount` 0))))

(fn `OnRep_PhysicsEnabled`
  (bind _weapon (`self.Weapon`))
  (bind _physicsenabled (`self.PhysicsEnabled`))
  (`PrimitiveComponent.SetSimulatePhysics` _weapon _physicsenabled)
  (if _physicsenabled
    (`PrimitiveComponent.SetCollisionEnabled` _weapon "QueryAndPhysics")
    (else
      (`PrimitiveComponent.SetCollisionEnabled` _weapon "NoCollision"))))

(fn `OnRep_ShootToLocation`)

(fn `Reload`
  (`/Engine/EditorBlueprintResources/ActorMacros.Switch Has Authority`
    (:`Authority`
      (set `self.CurrentAmmo` (`self.MaxAmmo`))
      (set `self.IsReloading` false))))

(fn `Set Fire Mode Burst`
  (if (`self.Burst`)
    (`self.SetFireMode` "NewEnumerator1")
    (else
      (`self.Set Fire Mode FullAuto`))))

(fn `Set Fire Mode FullAuto`
  (if (`self.FullAuto`)
    (`self.SetFireMode` "NewEnumerator2")
    (else
      (`self.Set Fire Mode Burst`))))

(fn `SetAimRecoil`
  (params (Aiming :type Boolean))
  (if Aiming
    (if (not (`self.AimRecoilEnabled`))
      (set `self.VerticalKick` (/ (`self.VerticalKick`) 2.0))
      (set `self.HorisontalKick` (/ (`self.HorisontalKick`) 2.0))
      (set `self.AimRecoilEnabled` true))
    (elif (`self.AimRecoilEnabled`)
      (set `self.VerticalKick` (* (`self.VerticalKick`) 2.0))
      (set `self.HorisontalKick` (* (`self.HorisontalKick`) 2.0))
      (set `self.AimRecoilEnabled` false))))

(fn `SetFireMode`
  (params (Firemode :type "/Game/RealisticBlueprintWeapons/Blueprints/FireModes Enum" :default "NewEnumerator0"))
  (`/Engine/EditorBlueprintResources/ActorMacros.Switch Has Authority`
    (:`Authority`
      (switch `/Game/RealisticBlueprintWeapons/Blueprints/FireModes` Firemode
        (:`NewEnumerator0`
          (if (`self.SingleShot`)
            (set `self.CurrentFireMode` Firemode :!label _label)))
        (:`NewEnumerator1`
          (if (`self.Burst`)
            (goto _label)))
        (:`NewEnumerator2`
          (if (`self.FullAuto`)
            (goto _label)))))
    (:`Remote`
      (switch `/Game/RealisticBlueprintWeapons/Blueprints/FireModes` Firemode
        (:`NewEnumerator0`
          (if (`self.SingleShot`)
            (set `self.CurrentFireMode` Firemode :!label _label_2)))
        (:`NewEnumerator1`
          (if (`self.Burst`)
            (goto _label_2)))
        (:`NewEnumerator2`
          (if (`self.FullAuto`)
            (goto _label_2)))))))

(fn `SetFireModeSingle`
  (if (`self.SingleShot`)
    (`self.SetFireMode` "NewEnumerator0")
    (else
      (`self.Set Fire Mode Burst`))))

(fn `SetIsJammed`
  (params (IsJammed :type Boolean))
  (`/Engine/EditorBlueprintResources/ActorMacros.Switch Has Authority`
    (:`Authority`
      (set `self.IsJammed` IsJammed))))

(fn `SetIsTriggerPulled`
  (params (TriggerPulled :type Boolean))
  (set `self.TriggerPulled` TriggerPulled))

(fn `SetRecoil`
  (bind _verticalkick (`self.GetVerticalKick`))
  (bind _output_get (set `self.TargetVerticalRecoil` _verticalkick))
  (bind _horisontalkick (`self.GetHorisontalKick`))
  (bind _output_get_2 (set `self.TargetHorisontalRecoil` _horisontalkick))
  (`self.RecoilApplied` _output_get _output_get_2))

(fn `TriggerNoAmmo`
  (`KismetSystemLibrary.PrintString` "No ammo, CLICK!")
  (set `self.TriggerPulled` false)
  ;[1 1 1] This is done to prevent burst completing after reload
  (set `self.CurrentShotInBurst` 9000))

(fn `Try Spawn Projectile`
  (bind _visibleprojectile_replicate_to_clients_ (`self.VisibleProjectile(replicate to clients)`))
  (bind _blastprojectilecount (`self.BlastProjectileCount`))
  (bind (_x _y) (`KismetMathLibrary.BreakVector2D` (`self.HorisontalSpread`)))
  (bind (_x_2 _y_2) (`KismetMathLibrary.BreakVector2D` (`self.VerticalSpread`)))
  (`self.FindMuzzle`)
  (`/Engine/EditorBlueprintResources/ActorMacros.Switch Has Authority`
    (:`Authority`
      (`self.WillItJam`)
      (if (`self.IsJammed`)
        ;[1 1 1] If you want to do something while jammed, do it here
        (`KismetSystemLibrary.PrintString` "Jammed!")
        (else
          (set `self.TimeSinceLastShot` 0.0)
          (set `self.CurrentAmmo` (- (`self.CurrentAmmo`) 1))
          (`self.ShotCosmetics`)
          ;[1 1 1] Setting all the variables of the projectile
          (`self.SetRecoil`)
          (bind _returnvalue (`|SpawnActorFromClass` "/Game/Sandbox/Weapons/WeaponSystems/Projectile.Projectile_C" (`self.MuzzleSocketTransform`) "AdjustIfPossibleButDontSpawnIfColliding" "OverrideRootScale" null (* (`KismetMathLibrary.Normal` (+ (`self.ShotForwardVector`) (`KismetMathLibrary.GreaterGreater_VectorRotator` (`KismetMathLibrary.MakeVector` 0.0 (`KismetMathLibrary.RandomFloatInRange` (/ _x_2 1000.0) (/ _y_2 1000.0)) (`KismetMathLibrary.RandomFloatInRange` (/ _x 1000.0) (/ _y 1000.0))) (`self.ShotForwardRotation`)) (`KismetMathLibrary.GreaterGreater_VectorRotator` (`KismetMathLibrary.MakeVector` 0.0 0.0 (/ (`.Value_5_5991169347FC465AFEA0F8A0106A742B` (break `/Game/RealisticBlueprintWeapons/Blueprints/Weapons/ZeroingValue` (`self.ZeroingValue`))) 1000.0)) (`self.ShotForwardRotation`)))) (`self.MuzzleVelocity`)) (`self.BulletMass`) (`self.DestroyOnImpact`) (`self.Drag`) (`self.CaliberDiameter`) (`self.DoesRicochet`) (`self.BaseDamage`) (`self.ProjectileMesh`) (`self.ImpactEffect`) (`self.DebugTrace`) :!label _label))
          (`self.SetLifeSpan` _returnvalue (`self.ProjectileLifeSpan`))
          (`self.SetReplicates` _returnvalue _visibleprojectile_replicate_to_clients_)
          (`self.SetReplicateMovement` _returnvalue _visibleprojectile_replicate_to_clients_)
          ;[1 1 1] Blast loop code
          (if (and (> _blastprojectilecount 0) (< (`self.CurrentBlastCount`) _blastprojectilecount))
            (set `self.CurrentBlastCount` (+ (`self.CurrentBlastCount`) 1))
            (goto _label)
            (else
              (set `self.CurrentBlastCount` 0))))))))

(fn `UserConstructionScript`)

(fn `WillItJam`
  (if (not (`self.IsJammed`))
    (set `self.IsJammed` (> (`self.JamRisk`) (`KismetMathLibrary.RandomFloatInRange` 0.0 100.0)))))