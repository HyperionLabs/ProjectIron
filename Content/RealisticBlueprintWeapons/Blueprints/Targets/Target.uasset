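; Shooting target actor that changes to a random color when it takes damage and displays its world X position in meters.
; The construction script creates a dynamic material instance and writes the floored X distance to a text render.
; Damage sets the RepNotify Color variable to a random unit vector, and its OnRep applies that to the material's Color parameter.
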(event `self.ReceiveAnyDamage`
  (params (Damage :type "Float (single-precision)") (DamageType :type "DamageType Object Reference") (InstigatedBy :type "Controller Object Reference") (DamageCauser :type "Actor Object Reference"))
  (`self.ChangeColor`))

(fn `ChangeColor`
  (set `self.Color` (`KismetMathLibrary.RandomUnitVector`)))

(fn `OnRep_Color`
  (`MaterialInstanceDynamic.SetVectorParameterValue` (`self.Material`) "Color" (`KismetMathLibrary.Conv_VectorToLinearColor` (`self.Color`))))

(fn `UserConstructionScript`
  (bind _returnvalue (`PrimitiveComponent.CreateDynamicMaterialInstance` (`self.Target`) 0 "/Game/RealisticBlueprintWeapons/Materials/Colored.Colored"))
  (set `self.Material` _returnvalue)
  (`TextRenderComponent.K2_SetText` (`self.TextRender1`) (`KismetTextLibrary.Conv_IntToText` (`KismetMathLibrary.FFloor` (/ (.x (`self.K2_GetActorLocation`)) 100.0)))))